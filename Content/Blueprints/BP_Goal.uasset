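; BP_Goal is a level goal actor that ends the game when BP_player overlaps its Box component.
; On overlap it switches input to UI only, shows the mouse cursor and pauses the game.
; It then displays WBP_EndScreen, choosing between two ending types by whether the player's TrashCount is above zero.
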(event `self.Box.OnComponentBeginOverlap`
  (params (OverlappedComponent :type "PrimitiveComponent Object Reference") (OtherActor :type "Actor Object Reference") (OtherComp :type "PrimitiveComponent Object Reference") (OtherBodyIndex :type Integer) (bFromSweep :type Boolean) (SweepResult :type "HitResult Structure (by ref)"))
  (bind _returnvalue (`GameplayStatics.GetPlayerController` 0))
  (bind _asbp_player (cast `/Game/Blueprints/BP_player` OtherActor))
  (`WidgetBlueprintLibrary.SetInputMode_UIOnlyEx` _returnvalue null)
  (set `PlayerController.bShowMouseCursor` true _returnvalue)
  (if (> (`/Game/Blueprints/BP_player.TrashCount` _asbp_player) 0)
    (`GameplayStatics.SetGamePaused` true)
    (bind _returnvalue_2 (`|CreateWidget` "/Game/Widgets/WBP_EndScreen.WBP_EndScreen_C"))
    (`UserWidget.AddToViewport` _returnvalue_2 0)
    (else
      (`GameplayStatics.SetGamePaused` true)
      (bind _returnvalue_3 (`|CreateWidget` "/Game/Widgets/WBP_EndScreen.WBP_EndScreen_C" null 1))
      (`UserWidget.AddToViewport` _returnvalue_3 0))))

(fn `UserConstructionScript`)