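; BP_buoy is a bumper-style buoy that knocks away whatever hits its capsule.
; On a hit, a look-at direction from the buoy to the other actor launches BP_player along it, overriding velocity, and plays a one-shot buoy animation.
; Other hit components get a pushing force in that direction instead, and every hit calls a play-sound at the buoy's location.
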(event `self.Capsule.OnComponentHit`
  (params (HitComponent :type "PrimitiveComponent Object Reference") (OtherActor :type "Actor Object Reference") (OtherComp :type "PrimitiveComponent Object Reference") (NormalImpulse :type "Vector Structure") (Hit :type "HitResult Structure (by ref)"))
  (bind _returnvalue (`KismetMathLibrary.Conv_RotatorToVector` (`KismetMathLibrary.FindLookAtRotation` (`self.K2_GetActorLocation`) (`self.K2_GetActorLocation` OtherActor))))
  (bind _asbp_player (cast `/Game/Blueprints/BP_player` OtherActor)
    (:`then`
      (`Character.LaunchCharacter` _asbp_player (* _returnvalue 1300.0) true true)
      (`SkeletalMeshComponent.PlayAnimation` (`self.SkeletalMesh`) "/Game/Geometry/Buoy/Buoy_01a_Anim.Buoy_01a_Anim" false))
    (:`CastFailed`
      (`PrimitiveComponent.AddForce` OtherComp (* _returnvalue 5000.0) "None" false)))
  (`GameplayStatics.PlaySoundAtLocation` null (`self.K2_GetActorLocation`) (struct) 1.0 1.0 0.0 null null null))

(fn `UserConstructionScript`)