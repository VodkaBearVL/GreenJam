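; BP_SpawnArea is an actor that spawns items within a box area and also runs the game's countdown to the end screen.
; Each Tick spawns a BP_item at a random point in the Box bounds whenever a randomly re-rolled delay runs out.
; When TimeLimit expires, it pauses the game, switches to UI input and shows WBP_EndScreen, choosing the ending by whether the player's TrashCount is above zero.
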(event `self.ReceiveTick`
  (params (DeltaSeconds :type "Float (single-precision)"))
  (bind _returnvalue (`GameplayStatics.GetPlayerController` 0))
  (bind (_origin _boxextent) (`KismetSystemLibrary.GetComponentBounds` (`self.Box`)))
  (`|ExecutionSequence`
    (:`then_0`
      (set `self.Timer` (+ DeltaSeconds (`self.Timer`)))
      (bind _output_get (set `self.TimeLimit` (- (`self.TimeLimit`) DeltaSeconds)))
      (if (<= (`self.TimeToSpawm`) 0.0)
        (`|SpawnActorFromClass` "/Game/Blueprints/BP_item.BP_item_C" (`KismetMathLibrary.Conv_VectorToTransform` (`KismetMathLibrary.RandomPointInBoundingBox` _origin _boxextent)) "Undefined" "OverrideRootScale" null null)
        (set `self.TimeToSpawm` (`KismetMathLibrary.RandomFloatInRange` 0.0 5.0))
        (else
          (set `self.TimeToSpawm` (- (`self.TimeToSpawm`) DeltaSeconds)))))
    (:`then_1`
      (if (<= _output_get 0.0)
        (`GameplayStatics.SetGamePaused` true)
        (`WidgetBlueprintLibrary.SetInputMode_UIOnlyEx` _returnvalue null)
        (set `PlayerController.bShowMouseCursor` true _returnvalue)
        (bind _asbp_player (cast `/Game/Blueprints/BP_player` (`GameplayStatics.GetPlayerCharacter` 0)))
        (if (> (`/Game/Blueprints/BP_player.TrashCount` _asbp_player) 0)
          (bind _returnvalue_2 (`|CreateWidget` "/Game/Widgets/WBP_EndScreen.WBP_EndScreen_C" null 2))
          (`UserWidget.AddToViewport` _returnvalue_2 0)
          (else
            (bind _returnvalue_3 (`|CreateWidget` "/Game/Widgets/WBP_EndScreen.WBP_EndScreen_C" null 3))
            (`UserWidget.AddToViewport` _returnvalue_3 0)))))))

(fn `UserConstructionScript`)