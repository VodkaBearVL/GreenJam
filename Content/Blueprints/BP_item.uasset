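; BP_item is a litter item actor that appears as one of six random plastic-waste style props, such as a straw, bag or bottle.
; The construction script picks the static mesh at random.
; On BeginPlay, Sphere receives a strong one-off push along world negative X, applied as an acceleration change.
; Each Tick moves the mesh to the sphere's location, copying position but not rotation.
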(event `self.ReceiveTick`
  (params (DeltaSeconds :type "Float (single-precision)"))
  (`SceneComponent.K2_SetWorldLocation` (`self.StaticMesh`) (`SceneComponent.K2_GetComponentLocation` (`self.Sphere`)) false false))

(event `self.ReceiveBeginPlay`
  (`PrimitiveComponent.AddForce` (`self.Sphere`) (-50000.0 0.0 0.0) "None" true))

(fn `UserConstructionScript`
  (switch `int` (`KismetMathLibrary.RandomIntegerInRange` 0 5)
    (:`0`
      (`StaticMeshComponent.SetStaticMesh` (`self.StaticMesh`) "/Game/Static_Meshes/SM_Tooth_Brush_A1_ML.SM_Tooth_Brush_A1_ML"))
    (:`1`
      (`StaticMeshComponent.SetStaticMesh` (`self.StaticMesh`) "/Game/Static_Meshes/SM_Can_Holder_A1_ML.SM_Can_Holder_A1_ML"))
    (:`2`
      (`StaticMeshComponent.SetStaticMesh` (`self.StaticMesh`) "/Game/Static_Meshes/SM_Ear_Bud_A1_ML.SM_Ear_Bud_A1_ML"))
    (:`3`
      (`StaticMeshComponent.SetStaticMesh` (`self.StaticMesh`) "/Game/Static_Meshes/SM_Plastic_Bag_A1_ML.SM_Plastic_Bag_A1_ML"))
    (:`4`
      (`StaticMeshComponent.SetStaticMesh` (`self.StaticMesh`) "/Game/Static_Meshes/SM_Straw_A1_ML.SM_Straw_A1_ML"))
    (:`5`
      (`StaticMeshComponent.SetStaticMesh` (`self.StaticMesh`) "/Game/Static_Meshes/SM_Milk_Bottle_A1_ML.SM_Milk_Bottle_A1_ML"))))